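; Enemy AI pawn that patrols, chases the player and is destroyed when damage depletes its Health.
; Tick moves it to random nearby reachable points after random delays while CanSeeEnemy is false.
; PawnSensing sightings of BP_Player set that flag and start a chase, with a retriggerable delay clearing it shortly after sightings stop.
; Line-trace-aimed BP_Projectile firing from the cannon socket exists but is disconnected, so it never runs.
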(event OnSeePawn(PawnSensing)
  (params (Pawn :type Pawn%20Object%20Reference))
  ;[1 1 1] AI follow player if detected
  (bind _asbp_player (Utilities|Casting|CastToBP_Player Pawn))
  (Utilities|FlowControl|Sequence
    (:then_0
      (Variables|Default|SetCanSeeEnemy? true)
      (AI|AIMoveTo self "0, 0, 0" _asbp_player 5.0 false))
    (:then_1
      (Utilities|FlowControl|RetriggerableDelay 0.5)
      (Variables|Default|SetCanSeeEnemy? false))))

(event EventTick
  (params (DeltaSeconds :type Float%20%28single-precision%29))
  ;[1 1 1] AI patrols at random position / Return to patrols if player not visible
  (if (not (Variables|Default|GetCanSeeEnemy?))
    (Utilities|FlowControl|Delay (Math|Random|RandomFloatinRange 2.0 5.0))
    (AI|AIMoveTo self (.RandomLocation (AI|Navigation|GetRandomReachablePointinRadius (Transformation|GetActorLocation) 3.5e+02 0 0)) 0 5.0 false)))

(event Game|Damage|EventAnyDamage
  (params (Damage :type Float%20%28single-precision%29) (DamageType :type Damage%20Type%20Object%20Reference) (InstigatedBy :type Controller%20Object%20Reference) (DamageCauser :type Actor%20Object%20Reference))
  ;[1 1 1] Enemy take damage
  (Variables|Default|SetHealth (- (Variables|Default|GetHealth) Damage))
  (if (<= (Variables|Default|GetHealth) 0.0)
    (Actor|DestroyActor)))

(fn ConstructionScript)